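; Battery pickup Blueprint that plays an electric-arc effect between the battery and the player when collected.
; WasCollected flags the battery as collecting and attaches two beam emitters to the pickup mesh.
; A short Delay loop keeps re-aiming the beam ends at two sockets on the player's mesh, so the arcs follow the character.
; After a one-second delay, it calls the parent WasCollected logic.
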(event EventWasCollected
  (bind _returnvalue (Game|GetPlayerCharacter 0))
  (bind _pickupmesh (Variables|Default|GetPickupMesh))
  (bind _mesh (Variables|/Script/Engine.Character|GetMesh _returnvalue))
  ;[1 1 1] Particle effects when collecting
  (Class|BatteryPickup|BatteryUpdateCollecting true)
  (bind _returnvalue_2 (Effects|SpawnEmitterAttached "/Game/ParticleSystems/P_electricity_arc.P_electricity_arc" _pickupmesh "None" "0, 0, 0" "0, 0, 0" "SnapToTargetIncludingScale"))
  (bind _returnvalue_3 (Effects|SpawnEmitterAttached "/Game/ParticleSystems/P_electricity_arc.P_electricity_arc" _pickupmesh "None" "0, 0, 0" "0, 0, 0" "SnapToTargetIncludingScale"))
  (Class|ParticleSystemComponent|SetBeamTargetPoint _returnvalue_2 0 (Transformation|GetSocketLocation _mesh "joint40") :!label _label)
  (Class|ParticleSystemComponent|SetBeamTargetPoint _returnvalue_3 0 (Transformation|GetSocketLocation _mesh "joint25") :!label _label_2)
  (Utilities|FlowControl|Sequence
    (:then_0
      (Utilities|FlowControl|Sequence
        (:then_0
          (Utilities|FlowControl|Delay 1.0)
          (|CallParentFunction))
        (:then_1
          (Utilities|FlowControl|Delay 0.05)
          (goto _label))))
    (:then_1
      (Utilities|FlowControl|Sequence
        (:then_0
          (Utilities|FlowControl|Delay 1.0))
        (:then_1
          (Utilities|FlowControl|Delay 0.05)
          (goto _label_2))))))

(fn ConstructionScript)